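; Elevator door button that opens or operates the elevator gate when the player character interacts with it.
; On Interacts from a BP_MysteryChar, it prints a debug message, finds a BP_ElevatorGate2 through GetActorOfClass and calls GateActivated.
; CanInteract? always returns false.
; The FlipFlop toggle for gate deactivation and the timeline for moving the pushed button are disconnected and never run.
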(event `/Game/Blueprints/Interfaces/BPI_Interacts.Interacts`
  (params (interactionActor :type "Character Object Reference"))
  (cast `/Game/Blueprints/GAME/BP_MysteryChar` interactionActor)
  (`KismetSystemLibrary.PrintString` "buttonpressed")
  (bind _returnvalue (`GameplayStatics.GetActorOfClass` "/Game/Blueprints/Switches/BP_ElevatorGate2.BP_ElevatorGate2_C"))
  (`/Engine/EditorBlueprintResources/StandardMacros.IsValid` _returnvalue
    (:`Is Valid`
      (`/Game/Blueprints/Switches/BP_ElevatorGate2.GateActivated` _returnvalue))))

(fn `CanInteract?`
  (returns (`Interactable?` :type Boolean))
  (return false))

(fn `UserConstructionScript`)