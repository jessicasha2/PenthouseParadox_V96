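; Elevator gate Blueprint that toggles open or closed on GateActivated by animating the actor's X scale with a Timeline.
; IsDoorOpen selects forward or reverse playback, IsDoorActive blocks retriggering mid-animation, and a FlipFlop updates the open state on finish.
; GateDeactivated only prints and decrements the switch counter; its threshold check drives nothing, and the counter's increment logic is disconnected.
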(event `GateActivated`
  (`KismetSystemLibrary.PrintString` "gateActivated")
  (if (not (`self.isDoorActive`))
    (set `self.isDoorActive` true)
    (if (`self.isDoorOpen?`)
      (bind (_direction _alpha) (`Timeline|Timeline` :!via `ReverseFromEnd` :!label _label)
        (:`Update`
          (`self.SetActorScale3D` (`KismetMathLibrary.MakeVector` _alpha 1.0 1.0)))
        (:`Finished`
          (set `self.isDoorActive` false)
          (`/Engine/EditorBlueprintResources/StandardMacros.FlipFlop`
            (:`A`
              (set `self.isDoorOpen?` true))
            (:`B`
              (set `self.isDoorOpen?` false)))))
      (else
        (goto _label :!via `PlayFromStart`)))))

(event `GateDeactivated`
  (`KismetSystemLibrary.PrintString` "gateDeactivated")
  (`/Engine/EditorBlueprintResources/StandardMacros.DecrementInt` (`self.Num Switch Activated`)
    (:`  `
      (if (>= (`self.Num Switch Activated`) (`self.Num Switches Needed`))
        _))))

(fn `UserConstructionScript`)