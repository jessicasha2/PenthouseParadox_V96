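; BP_HiddenDoor is a switch-driven door that moves its Barrier component once enough switches are active.
; BarrierActivated and BarrierDeactivated adjust an active-switch count and compare it to NumSwitchesNeeded, playing Barrier_TL when met and reversing it otherwise.
; The timeline's Alpha output directly sets the barrier's relative Z location.
; A delayed BarrierDown_TL movement is left unconnected and never runs.
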(event `self.ReceiveTick`
  (params (DeltaSeconds :type "Float (single-precision)"))
  ;[1 1 1] debugging
)

(event `BarrierActivated`
  (`/Engine/EditorBlueprintResources/StandardMacros.IncrementInt` (`self.NumSwitchActivated`)
    (:`  `
      (if (>= (`self.NumSwitchActivated`) (`self.NumSwitchesNeeded`))
        (bind (_direction _alpha) (`Timeline|Barrier_TL` :!label _label)
          (:`Update`
            (`SceneComponent.K2_SetRelativeLocation` (`self.barrier`) (`KismetMathLibrary.MakeVector` 0.0 0.0 _alpha) false false)))
        (else
          (goto _label :!via `Reverse`))))))

(event `BarrierDeactivated`
  (`/Engine/EditorBlueprintResources/StandardMacros.DecrementInt` (`self.NumSwitchActivated`)
    (:`  `
      (if (>= (`self.NumSwitchActivated`) (`self.NumSwitchesNeeded`))
        (goto _label)
        (else
          (goto _label :!via `Reverse`))))))

(fn `UserConstructionScript`)