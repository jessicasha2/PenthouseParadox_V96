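; Player movement component that switches walk, sprint and crouch speeds on the character, with Sanity intended as the sprint stamina pool.
; Initialize stores the player reference, and sprint and crouch events set max walk speed.
; Looping function-name timers regenerate Sanity after a retriggerable delay when sprinting stops; SprintTimer drains it while moving.
; Work in progress: the sprint timer start is disconnected, and StopSprint and EndCrouch are empty.
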(event `StartSprinting`
  ;[0.6249 0.4297 1] Start Sprinting
  (`self.Set Max Walk Speed` (`self.SprintSpeed`)))

(event `SprintTimer`
  (if (and (> (`self.CurrentSanity`) (`self.MinSanity`)) (> (`KismetMathLibrary.VSize` (`Actor.GetVelocity` (`self.Player_REF`))) 10.0))
    ;[0.2299 0.6145 1] How long can you sprint?
    (bind _output_get (set `self.CurrentSanity` (`KismetMathLibrary.FClamp` (- (`self.CurrentSanity`) 1.0) (`self.MinSanity`) (`self.MaxSanity`))))
    (`KismetSystemLibrary.PrintString` (`KismetStringLibrary.Conv_DoubleToString` _output_get) false false)
    (if (<= (`self.CurrentSanity`) (`self.MinSanity`))
      (`self.StopSprint`))
    (else
      (`self.StopSprint`))))

(event `StopSprinting`
  ;[1 1 1] Stop Sprinting
  (if (not (`self.IsCrouching?`))
    (`KismetSystemLibrary.K2_ClearTimer` null "SprintTimer")
    (`self.Set Max Walk Speed` (`self.WalkSpeed`))
    (`KismetSystemLibrary.RetriggerableDelay` 5.0)
    (if (not (`KismetSystemLibrary.K2_IsTimerActive` null "SprintTimer"))
      ;[1 1 1] check this later
      (`KismetSystemLibrary.K2_SetTimer` null "RegenerateSanity" 0.03 true))))

(event `StartCrouch`
  (bind _crouchspeed (`self.CrouchSpeed`))
  ;[1 0.9359 0.09279] Work on crouch logic start Crouch never being called
  (`KismetSystemLibrary.PrintString` "startCrouch")
  (if (`self.IsCrouching?`)
    (`self.EndCrouch`))
  (`KismetSystemLibrary.K2_ClearTimer` null "SprintTimer")
  (`KismetSystemLibrary.PrintString` (`KismetStringLibrary.Conv_DoubleToString` (`self.WalkSpeed`)))
  (`KismetSystemLibrary.PrintString` (`KismetStringLibrary.Conv_DoubleToString` (`self.SprintSpeed`)))
  (`self.Set Max Walk Speed` _crouchspeed)
  (`KismetSystemLibrary.PrintString` (`KismetStringLibrary.Conv_DoubleToString` _crouchspeed)))

(event `EndCrouch`
  ;[1 0.9359 0.09279] Work on crouch logic start Crouch never being called
)

(event `RegenerateSanity`
  ;[0.926 0.4855 1] Sanity Regenerations, if only this worked in real life
  (bind _output_get (set `self.CurrentSanity` (`KismetMathLibrary.FClamp` (+ (`self.CurrentSanity`) 1.0) (`self.MinSanity`) (`self.MaxSanity`))))
  (`KismetSystemLibrary.PrintString` (`KismetStringLibrary.Conv_DoubleToString` _output_get))
  (if (>= (`self.CurrentSanity`) (`self.MaxSanity`))
    (`KismetSystemLibrary.K2_ClearTimer` null "RegenerateSanity")))

(fn `Initialize`
  (params (Player_REF :type "/Game/Blueprints/GAME/BP_MysteryChar Object Reference"))
  (bind _output_get (set `self.Player_REF` Player_REF))
  (set `CharacterMovementComponent.MaxWalkSpeed` (`self.WalkSpeed`) (`Character.CharacterMovement` _output_get)))

(fn `Set Max Walk Speed`
  (params (MaxWalkSpeed :type "Float (single-precision)")))

(fn `SetMaxWalkSpeed`
  (params (MaxWalkSpeed :type "Float (double-precision)"))
  (set `CharacterMovementComponent.MaxWalkSpeed` MaxWalkSpeed (`Character.CharacterMovement` (`self.Player_REF`))))

(fn `StopSprint`)