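; Flashlight component that tracks battery charge and whether the battery is dead.
; DecreaseBattery and IncreaseBattery adjust the charge, clamp it between minimum and maximum and return the new value.
; Draining to the minimum sets IsBatDead, while any call to IncreaseBattery clears it without checking the level.
; It has no active events and does not touch a light itself, only holding battery state.
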(fn `DecreaseBattery`
  (params (DrainBat :type "Float (double-precision)"))
  (returns (CurrentBat :type "Float (double-precision)"))
  (bind _output_get (set `self.CurrentFLBat` (`KismetMathLibrary.FClamp` (- (`self.CurrentFLBat`) DrainBat) (`self.MinFLBat`) (`self.MaxFLBat`))))
  (if (<= (`self.CurrentFLBat`) (`self.MinFLBat`))
    ;[1 1 1] BatteryDead no spotlight visibility
    (set `self.isBatDead?` true)
    (return _output_get)
    (else
      (set `self.isBatDead?` false)
      (return _output_get))))

(fn `IncreaseBattery`
  (params (IcreaseBat :type "Float (double-precision)"))
  (returns (CurrentBat :type "Float (double-precision)"))
  (bind _output_get (set `self.CurrentFLBat` (`KismetMathLibrary.FClamp` (+ IcreaseBat (`self.CurrentFLBat`)) (`self.MinFLBat`) (`self.MaxFLBat`))))
  ;[1 1 1] Return Abiliity to use Flashlight
  (set `self.isBatDead?` false)
  (return _output_get))